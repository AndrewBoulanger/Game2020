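; BP_CoolerCar is a player-driven vehicle that can shoot, with forward and right axes feeding throttle and steering on its VehicleMovement component.
; Fire spawns a Player_Bullet at the Coneeeeeee component's transform and passes the car's velocity to the bullet's SetSpeed.
; Tab rights the car by teleporting its rotation to keep only the current yaw.
; The quit action adds a UI_MM_QuitGame widget to the viewport.
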(event EventBeginPlay)

(event Collision|EventActorBeginOverlap
  (params (OtherActor :type Actor%20Object%20Reference)))

(event EventTick
  (params (DeltaSeconds :type Float%20%28single-precision%29)))

(event Input|ActionEvents|InputActionquit
  (params (Key :type Key%20Structure :default "None"))
  (:Pressed
    (bind _returnvalue (UserInterface|CreateWidget "/Game/UI_Blueprints/UI_MM_QuitGame.UI_MM_QuitGame_C" (Game|GetPlayerController 0)))
    (UserInterface|Viewport|AddtoViewport _returnvalue 0)))

(event Input|ActionEvents|InputActionFire
  (params (Key :type Key%20Structure :default "None"))
  (:Pressed
    (bind _returnvalue (Game|SpawnActorfromClass "/Game/Blueprints/Player_Bullet.Player_Bullet_C" (Transformation|GetWorldTransform (Variables|Default|GetConeeeeeee)) "AlwaysSpawn" 0 0))
    (Default|SetSpeed _returnvalue (Transformation|GetVelocity))))

(event Input|AxisEvents|InputAxisforward
  (params (AxisValue :type Float%20%28single-precision%29))
  (Class|WheeledVehicleMovementComponent|SetThrottleInput (Variables|Default|GetVehicleMovement) AxisValue))

(event Input|AxisEvents|InputAxisright
  (params (AxisValue :type Float%20%28single-precision%29))
  (Class|WheeledVehicleMovementComponent|SetSteeringInput (Variables|Default|GetVehicleMovement) AxisValue))

(event Input|KeyboardEvents|Tab
  (params (Key :type Key%20Structure :default "None"))
  (:Pressed
    (Transformation|SetActorRotation (Math|Rotator|MakeRotator 0.0 0.0 (.yaw (Transformation|GetActorRotation))) true)))

(fn ConstructionScript)