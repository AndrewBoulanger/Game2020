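; AI wheeled vehicle that drives toward a move target, while also accepting player throttle and steering axes and a debug health-damage key.
; ReceiveMoveTarget stores the target, releases the handbrake and, after a short delay, runs a single UpdateMovement pass.
; Steering maps yaw error to the target, adding a random offset at close range.
; The distance-based throttle formula is multiplied by zero and clamped with inverted bounds, so its output is constant.
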(event Custom|ReceiveMoveTarget
  (params (Target :type Vector))
  (CallFunction|MovetoLocation Target)
  (Utilities|FlowControl|Delay 0.1)
  (CallFunction|UpdateMovement))

(event EventBeginPlay
  (Input|EnableInput (Game|GetPlayerController 0)))

(event Collision|EventActorBeginOverlap
  (params (OtherActor :type Actor%20Object%20Reference)))

(event EventTick
  (params (DeltaSeconds :type Float%20%28single-precision%29)))

(event Input|AxisEvents|InputAxisforward
  (params (AxisValue :type Float%20%28single-precision%29))
  (Class|WheeledVehicleMovementComponent|SetThrottleInput (Variables|Default|GetVehicleMovement) AxisValue))

(event Input|AxisEvents|InputAxisright
  (params (AxisValue :type Float%20%28single-precision%29))
  (Class|WheeledVehicleMovementComponent|SetSteeringInput (Variables|Default|GetVehicleMovement) AxisValue))

(event Input|KeyboardEvents|L
  (params (Key :type Key%20Structure))
  (:Pressed
    (Variables|Default|SetHealthCurr (- (Variables|Default|GetHealthCurr) 2e+01))))

(fn ConstructionScript)

(fn MovetoLocation
  (params (TargetLocation :type Vector))
  (Variables|Default|Settarget TargetLocation)
  (Variables|Default|SetInitialDistance (Math|Vector|VectorLength (- (Transformation|GetActorLocation) (Variables|Default|Gettarget))))
  (Variables|Default|SetStartingTime (Utilities|Time|GetGameTimeinSeconds))
  (Class|WheeledVehicleMovementComponent|SetHandbrakeInput (Variables|Default|GetVehicleMovement) false))

(fn UpdateMovement
  (bind _returnvalue (Transformation|GetActorLocation))
  (bind _returnvalue_2 (Transformation|GetActorRotation))
  (bind _target (Variables|Default|Gettarget))
  (bind _returnvalue_3 (Math|Rotator|FindLookatRotation _returnvalue _target))
  (bind _returnvalue_4 (Math|Rotator|Delta(Rotator) _returnvalue_3 _returnvalue_2))
  (bind _yaw (Math|Rotator|BreakRotator _returnvalue_4))
  (LocalVariables|SetCurrentLocationLocal _returnvalue)
  (Class|WheeledVehicleMovementComponent|SetSteeringInput (Variables|Default|GetVehicleMovement) (Math|Float|MapRangeUnclamped (Math|Float|SelectFloat _yaw (+ _yaw (* (Math|Float|Sign(Float) _yaw) (Math|Random|RandomFloatinRange -9e+01 -45.0))) (> (Math|Vector|VectorLength (- (Variables|Default|Gettarget) (LocalVariables|GetCurrentLocationLocal))) 1.5e+03)) -1.8e+02 1.8e+02 -1.0 1.0))
  (bind _output_get (LocalVariables|SetCurrent%20Distance%20Local (Math|Vector|VectorLength (- (LocalVariables|GetCurrentLocationLocal) (Variables|Default|Gettarget)))))
  (bind _output_get_2 (LocalVariables|SetCurrent%20Input%20Local (Math|Float|Clamp(Float) (* (Math|Float|Power (- _output_get (Utilities|Time|GetGameTimeinSeconds)) (+ (* _output_get 2.5e-05) 1.0)) 0.0) 1e+01 -1e+01)))
  (Class|WheeledVehicleMovementComponent|SetThrottleInput (Variables|Default|GetVehicleMovement) _output_get_2))