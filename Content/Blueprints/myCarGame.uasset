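; myCarGame is a car game manager Blueprint that sets up the UI and steers AI cars toward the player's car.
; BeginPlay creates the UI widget for player 0 and adds it to the viewport.
; Every Tick it looks up the BP_CoolerCar and all BP_AI_Car actors, records their count in NumberOfCPUs, and passes the cooler car's location to each AI through ReceiveMoveTarget.
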(event EventBeginPlay
  (bind _returnvalue (UserInterface|CreateWidget "/Game/Blueprints/UI.UI_C" (Game|GetPlayerController 0)))
  (UserInterface|Viewport|AddtoViewport _returnvalue 0))

(event EventTick
  (params (DeltaSeconds :type Float%20%28single-precision%29))
  (bind _returnvalue (Actor|GetActorOfClass "/Game/Blueprints/BP_CoolerCar.BP_CoolerCar_C"))
  (bind _outactors (Actor|GetAllActorsOfClass "/Game/Blueprints/BP_AI_Car.BP_AI_Car_C"))
  (Variables|Default|SetNumber%20of%20CPUs (Utilities|Array|Length _outactors))
  (for _array_element _outactors
    (Default|ReceiveMoveTarget _array_element (Transformation|GetActorLocation _returnvalue))))

(fn ConstructionScript)