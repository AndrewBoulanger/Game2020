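; BP_orbiting_Sphere is a rotating hazard that damages and stuns the player's car on contact.
; Tick adds RotationSpeed to the actor's local pitch each frame, without delta-time scaling.
; Actor overlap checks for the "player" tag, casts to BP_CoolerCar and calls TakeDamage with damage, stun time and cooldown.
; An impulse call on the car's mesh is left unconnected and never runs.
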(event EventBeginPlay)

(event Collision|EventActorBeginOverlap
  (params (OtherActor :type Actor%20Object%20Reference))
  (Utilities|IsValid OtherActor
    (:Is%20Valid
      (if (Actor|ActorHasTag OtherActor "player")
        (bind _asbp_cooler_car (Utilities|Casting|CastToBP_CoolerCar OtherActor))
        (Default|TakeDamage _asbp_cooler_car 2e+02 4.0 true)))))

(event EventTick
  (params (DeltaSeconds :type Float%20%28single-precision%29))
  (Transformation|AddActorLocalRotation (Math|Rotator|MakeRotator 0.0 (Variables|Default|Getrotation%20speed) 0.0) false false))

(fn ConstructionScript)