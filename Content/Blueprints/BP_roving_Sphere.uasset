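; BP_roving_Sphere is a moving hazard that damages and stuns the player's car on contact.
; Each Tick increments Theta and feeds its sine into swept X/Y offsets on the root scaled by XDir and YDir, giving a frame-based back-and-forth motion, while pitching by RotationSpeed.
; Overlapping a "player"-tagged BP_CoolerCar calls its TakeDamage with fixed damage and stun time.
; An impulse node on the car's mesh is left unconnected.
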(event EventBeginPlay)

(event Collision|EventActorBeginOverlap
  (params (OtherActor :type Actor%20Object%20Reference))
  (if (Actor|ActorHasTag OtherActor "player")
    (bind _asbp_cooler_car (Utilities|Casting|CastToBP_CoolerCar OtherActor))
    (Default|TakeDamage _asbp_cooler_car 2e+02 4.0)))

(event EventTick
  (params (DeltaSeconds :type Float%20%28single-precision%29))
  (bind _result (Math|Float|IncrementFloat (Variables|Default|Gettheta))
    (:%20%20
      (Transformation|AddRelativeLocation (Variables|Default|GetDefaultSceneRoot) (Math|Vector|MakeVector (* (Math|Trig|Sin(Degrees) _result) (Variables|Default|GetXDir)) (* (Math|Trig|Sin(Degrees) _result) (Variables|Default|GetYDir)) 0.0) true false)
      (Transformation|AddActorLocalRotation (Math|Rotator|MakeRotator 0.0 (Variables|Default|Getrotation%20speed) 0.0) false false))))

(fn ConstructionScript)