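; Enemy turret that turns toward the player's car (BP_CoolerCar) and shoots at it when seen.
; PawnSensing drives everything: each sighting snaps the whole actor to face the car, then spawns an Enemy_Bullet at BulletSpawnpoint after a short Delay.
; The Delay ignores re-triggers while pending, so it also throttles the fire rate.
; The construction script sets the Turrent component's text from TextTingy.
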(event OnSeePawn(PawnSensing)
  (params (Pawn :type Pawn%20Object%20Reference))
  (bind _asbp_cooler_car (Utilities|Casting|CastToBP_CoolerCar Pawn))
  (Utilities|FlowControl|Sequence
    (:then_0
      (Transformation|SetActorRotation (Math|Rotator|FindLookatRotation (Transformation|GetActorLocation) (Transformation|GetActorLocation _asbp_cooler_car)) true))
    (:then_1
      (Utilities|FlowControl|Delay 0.5)
      (Game|SpawnActorfromClass "/Game/Blueprints/Enemy_Bullet.Enemy_Bullet_C" (Transformation|GetWorldTransform (Variables|Default|GetBullet_Spawnpoint)) "Undefined" 0 0))))

(event EventBeginPlay)

(event Collision|EventActorBeginOverlap
  (params (OtherActor :type Actor%20Object%20Reference)))

(event EventTick
  (params (DeltaSeconds :type Float%20%28single-precision%29)))

(fn ConstructionScript
  (Rendering|Components|TextRender|SetText (Variables|Default|GetTurrent) (Variables|Default|GetText_tingy)))