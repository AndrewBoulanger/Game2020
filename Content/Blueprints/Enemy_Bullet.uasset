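; Enemy projectile Blueprint that damages and stuns the player's car when it overlaps it.
; On overlap, an actor tagged Player is cast to BP_CoolerCar and receives the bullet's Damage value plus a fixed stun through TakeDamage.
; The bullet then destroys itself, as it does on overlapping any other actor or one already being destroyed, though a failed car cast leaves it alive.
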(event EventBeginPlay)

(event Collision|EventActorBeginOverlap
  (params (OtherActor :type Actor%20Object%20Reference))
  (if (Game|IsActorBeingDestroyed OtherActor)
    _
    (else
      (Variables|Default|Setother OtherActor)
      (if (Actor|ActorHasTag (Variables|Default|Getother) "Player")
        (bind _asbp_cooler_car (Utilities|Casting|CastToBP_CoolerCar (Variables|Default|Getother)))
        (Default|TakeDamage _asbp_cooler_car (Math|Conversions|ToFloat(Integer) (Variables|Default|GetDamage)) 2.0))))
  (Actor|DestroyActor))

(event EventTick
  (params (DeltaSeconds :type Float%20%28single-precision%29)))

(fn ConstructionScript)