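; Player-fired projectile that damages turrets and destroys AI cars on overlap.
; Overlap branches on the other actor's first tag: Enemy turrets take damage, Enemy Car spawns an explosion and destroys the car; other hits just destroy the bullet.
; SetSpeed adds the firing car's horizontal speed to MinSpeed when it exceeds that minimum, otherwise uses MinSpeed, setting both initial and max projectile speed.
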(event EventBeginPlay)

(event Collision|EventActorBeginOverlap
  (params (OtherActor :type Actor%20Object%20Reference))
  (Utilities|IsValid OtherActor
    (:Is%20Valid
      (Variables|Default|Setother OtherActor)
      (switch name (Utilities|Array|Get(acopy) (Variables|/Script/Engine.Actor|GetTags OtherActor))
        (:Default
          (Actor|DestroyActor))
        (:Enemy
          (bind _asturret (Utilities|Casting|CastToTurret (Variables|Default|Getother)))
          (Default|TakeDamage _asturret)
          (Actor|DestroyActor))
        (:enemyCar
          (Game|SpawnActorfromClass "/Game/Blueprints/Explosion.Explosion_C" (Math|Transform|MakeTransform (Transformation|GetActorLocation (Variables|Default|Getother)) "0, 0, 0" "1,1,1") "Undefined" 0 0)
          (bind _asbp_ai_car (Utilities|Casting|CastToBP_AI_Car (Variables|Default|Getother)))
          (Default|DestroyCar _asbp_ai_car)
          (Actor|DestroyActor))))
    (:Is%20Not%20Valid
      (Actor|DestroyActor))))

(event EventTick
  (params (DeltaSeconds :type Float%20%28single-precision%29)))

(fn ConstructionScript)

(fn SetSpeed
  (params (carVelocity :type Vector))
  (bind _returnvalue (Math|Vector|VectorLengthXY carVelocity))
  (bind _projectilemovement (Variables|Default|GetProjectileMovement))
  (bind _minspeed (Variables|Default|GetminSpeed))
  (bind _output_get (Variables|/Script/Engine.ProjectileMovementComponent|SetMaxSpeed _projectilemovement (Math|Float|SelectFloat (+ _returnvalue _minspeed) _minspeed (> _returnvalue (Variables|Default|GetminSpeed)))))
  (Variables|/Script/Engine.ProjectileMovementComponent|SetInitialSpeed _projectilemovement _output_get))