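; BP_Pylon is an electric hazard that periodically damages the player's BP_CoolerCar.
; The Sphere component's activated and deactivated events retrigger each other, looping between a wait parked far below and a timed live window with a Tesla sound.
; Overlap events track the Player tag, and Tick calls CheckActive to apply damage, with a brief stun and cooldown flag, while live and overlapped.
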(event OnComponentBeginOverlap(Sphere)
  (params (OverlappedComponent :type Primitive%20Component%20Object%20Reference) (OtherActor :type Actor%20Object%20Reference) (OtherComp :type Primitive%20Component%20Object%20Reference) (OtherBodyIndex :type Integer) (bFromSweep :type Boolean) (SweepResult :type Hit%20Result%20Structure%20%28by%20ref%29))
  (Variables|Default|SetOverlapping (Actor|ActorHasTag OtherActor "Player")))

(event OnComponentEndOverlap(Sphere)
  (params (OverlappedComponent :type Primitive%20Component%20Object%20Reference) (OtherActor :type Actor%20Object%20Reference) (OtherComp :type Primitive%20Component%20Object%20Reference) (OtherBodyIndex :type Integer))
  (Utilities|IsValid OtherActor
    (:Is%20Valid
      (if (Actor|ActorHasTag OtherActor "Player")
        (Variables|Default|SetOverlapping false)))))

(event OnComponentActivated(Sphere)
  (params (Component :type Actor%20Component%20Object%20Reference) (bReset :type Boolean))
  (Transformation|SetRelativeLocation (Variables|Default|GetSphere) "0, 0,-10000.000000" false false)
  (Utilities|FlowControl|Delay 9.0)
  (Transformation|SetRelativeLocation (Variables|Default|GetSphere) "0, 0,-48.000000" false false)
  (Variables|Default|SetIsActivate true)
  (Audio|SpawnSoundatLocation "/Game/Audio/teslaSound.teslaSound" (Transformation|GetActorLocation) "0, 0, 0" 3.0 5.0 0.0 0 0 false)
  (Utilities|FlowControl|Delay 6.0)
  (Variables|Default|SetIsActivate false)
  (Components|Activation|Deactivate (Variables|Default|GetSphere)))

(event OnComponentDeactivated(Sphere)
  (params (Component :type Actor%20Component%20Object%20Reference))
  (Components|Activation|Activate (Variables|Default|GetSphere) false))

(event EventBeginPlay
  (Components|Activation|Activate (Variables|Default|GetSphere) false))

(event Collision|EventActorBeginOverlap
  (params (OtherActor :type Actor%20Object%20Reference)))

(event EventTick
  (params (DeltaSeconds :type Float%20%28single-precision%29))
  (CallFunction|CheckActive)
  (bind _result (Math|Float|IncrementFloat (Variables|Default|Gettheta))
    (:%20%20
      (Variables|Default|Settheta 0.0))))

(fn ConstructionScript)

(fn CheckActive
  (if (Variables|Default|GetIsActivate)
    (if (Variables|Default|GetOverlapping)
      (bind _asbp_cooler_car (Utilities|Casting|CastToBP_CoolerCar (Game|Player|GetPlayerPawn 0)))
      (Default|TakeDamage _asbp_cooler_car 75.0 0.1 true))))