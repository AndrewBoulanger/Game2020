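; BP_CoolerCar is a player-driven vehicle that can shoot bullets.
; The forward and right input axes feed throttle and steering directly into its VehicleMovement component.
; Fire spawns a Bullet at the world transform of the Coneeeeeee component, regardless of collisions.
; Tab resets the car's rotation to zero, which rights it but also discards its heading.
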(event EventBeginPlay)

(event Collision|EventActorBeginOverlap
  (params (OtherActor :type Actor%20Object%20Reference)))

(event EventTick
  (params (DeltaSeconds :type Float%20%28single-precision%29)))

(event Input|ActionEvents|InputActionFire
  (params (Key :type Key%20Structure :default "None"))
  (:Pressed
    (Game|SpawnActorfromClass "/Game/Blueprints/bullet.bullet_C" (Transformation|GetWorldTransform (Variables|Default|GetConeeeeeee)) "AlwaysSpawn" 0 0)))

(event Input|AxisEvents|InputAxisforward
  (params (AxisValue :type Float%20%28single-precision%29))
  (Class|WheeledVehicleMovementComponent|SetThrottleInput (Variables|Default|GetVehicleMovement) AxisValue))

(event Input|AxisEvents|InputAxisright
  (params (AxisValue :type Float%20%28single-precision%29))
  (Class|WheeledVehicleMovementComponent|SetSteeringInput (Variables|Default|GetVehicleMovement) AxisValue))

(event Input|KeyboardEvents|Tab
  (params (Key :type Key%20Structure :default "None"))
  (:Pressed
    (Transformation|SetActorRotation "0, 0, 0")))

(fn ConstructionScript)